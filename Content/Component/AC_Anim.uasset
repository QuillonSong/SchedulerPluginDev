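; AC_Anim is an actor component that records transform keyframes for its owner when a UI button event fires.
; Two seconds after BeginPlay it finds the first WB_FunctionButton widget and binds CE_Click to its EDMove event.
; Each click creates a scheduler task if none is valid, then adds the owner's current transform at the SchedulerSubsystem's current time to parallel timestamp and transform arrays.
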(event `self.ReceiveBeginPlay`
  (`parent.ReceiveBeginPlay`)
  (`KismetSystemLibrary.Delay` 2.0)
  (bind _foundwidgets (`WidgetBlueprintLibrary.GetAllWidgetsOfClass` "/Game/UI/WB_FunctionButton.WB_FunctionButton_C" false))
  (add `/Game/UI/WB_FunctionButton.ED_Move` (`|GetArrayItem` _foundwidgets) (delegate `CE_Click`)))

(event `CE_Click`
  (`self.Task`
    (:`then`
      _)
    (:`else`
      (`self.CreateTask`)))
  (`/Game/Component/BPML_Component.M_AddKeyframe` (`self.Task`) (`SchedulerSubsystem.GetCurrentTime` (subsystem `SchedulerSubsystem`)) (`self.Timestamp`) (`Actor.GetTransform` (`self.Owner`)) (`self.Transform`)))
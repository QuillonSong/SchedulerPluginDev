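; AC_Base is a base actor component that registers a task with a scheduler subsystem on behalf of its owning actor.
; BeginPlay caches the owner.
; CreateTask asks the SchedulerSubsystem for a task under the component's task name and the owner's display name, with the component as task owner, and stores the result.
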(event `self.ReceiveBeginPlay`
  (set `self.Owner` (`self.GetOwner`)))

(fn `CreateTask`
  (bind _returnvalue (`SchedulerSubsystem.CreateTask` (subsystem `SchedulerSubsystem`) (`self.TaskName`) (`KismetSystemLibrary.GetDisplayName` (`self.Owner`)) self))
  (set `self.Task` _returnvalue)
  (return))
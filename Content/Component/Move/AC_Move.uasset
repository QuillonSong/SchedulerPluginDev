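; AC_Move is an actor component that keyframes and plays back its owner's location along a scheduler timeline.
; Two seconds after BeginPlay, it binds to the move event of the first WB_FunctionButton found.
; Each click creates a task if needed and records the location at the scheduler's current time in parallel Location and Timestamp arrays.
; ExecuteTask lerps the owner between neighbouring keyframes, while removal and destroy events maintain both arrays.
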(event `self.ReceiveBeginPlay`
  (`parent.ReceiveBeginPlay`)
  (`KismetSystemLibrary.Delay` 2.0)
  (bind _foundwidgets (`WidgetBlueprintLibrary.GetAllWidgetsOfClass` "/Game/UI/WB_FunctionButton.WB_FunctionButton_C" false))
  (add `/Game/UI/WB_FunctionButton.ED_Move` (`|GetArrayItem` _foundwidgets) (delegate `CE_Click`)))

(event `CE_Click`
  (`self.Task`
    (:`then`
      _)
    (:`else`
      (`self.CreateTask`)))
  (`/Game/Component/BPML_Component.M_AddKeyframe` (`self.Task`) (`SchedulerSubsystem.GetCurrentTime` (subsystem `SchedulerSubsystem`)) (`self.Timestamp`) (`Actor.K2_GetActorLocation` (`self.Owner`)) (`self.Location`)))

(event `TaskInterface.ExecuteTask`
  (params (Alpha :type "Float (double-precision)") (bIsForward :type Boolean) (ClipIndex :type "ClipIndex Structure"))
  (bind _location (`self.Location`))
  (`Actor.K2_SetActorLocation` (`self.Owner`) (`KismetMathLibrary.VLerp` (`|GetArrayItem` _location ClipIndex_LastIndex) (`|GetArrayItem` _location ClipIndex_NextIndex) Alpha) false false))

(event `TaskInterface.RemoveKeyframe`
  (params (KeyframeIndex :type Integer))
  (`KismetArrayLibrary.Array_Remove` (`self.Location`) KeyframeIndex)
  (`KismetArrayLibrary.Array_Remove` (`self.Timestamp`) KeyframeIndex))

(event `TaskInterface.DestroyTask`
  (set `self.Task` null)
  (`KismetArrayLibrary.Array_Clear` (`self.Location`))
  (`KismetArrayLibrary.Array_Clear` (`self.Timestamp`)))
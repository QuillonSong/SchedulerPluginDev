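; BP_EQ0 is an actor that glides from its starting position to a hardcoded world-space point, with no further gameplay purpose shown.
; BeginPlay enables ticking, and each Tick uses VInterpTo to ease the location toward that target without sweeping for collision.
; Once the actor is within a small tolerance of the target, it disables its own tick and stops just short of the exact point.
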(event `self.ReceiveBeginPlay`
  (`parent.ReceiveBeginPlay`)
  (`self.SetActorTickEnabled` true))

(event `self.ReceiveTick`
  (params (DeltaSeconds :type "Float (single-precision)"))
  (`self.K2_SetActorLocation` (`KismetMathLibrary.VInterpTo` (`self.K2_GetActorLocation`) (1000.0 1000.0 1000.0) DeltaSeconds 0.2))
  (if (== (`self.K2_GetActorLocation`) (1000.0 1000.0 1000.0) :`ErrorTolerance` 10.0)
    (`self.SetActorTickEnabled` false)))

(fn `UserConstructionScript`
  (`parent.UserConstructionScript`))